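; Surveillance camera actor that tracks players inside its cone and shows its state with a colored floor or area decal.
; Cone overlaps set or clear DetectedPlayer, and state changes tint a dynamic decal material green for Seeking, yellow for Analyzing and red for Alarm.
; Alarm fires an electric shock effect toward the player and spawns a burst on them, which Seeking hides again.
; OnRaiseAlarm calls an alarm dispatcher.
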(event `self.ReceiveBeginPlay`
  (`SceneComponent.SetVisibility` (`self.ElectricShock`) false false)
  (bind _returnvalue (`KismetMaterialLibrary.CreateDynamicMaterialInstance` "/Game/SurveillanceCamera/AreaMaterial.AreaMaterial"))
  (bind _output_get (set `self.DecalMaterial` _returnvalue))
  (`DecalComponent.SetDecalMaterial` (`self.Decal`) _output_get)
  (`MaterialInstanceDynamic.SetVectorParameterValue` (`self.DecalMaterial`) "Color" (struct :`G` 1.0 :`B` 0.08696 :`A` 1.0) :!label _label)
  (`self.EndShockPlayer`))

(event `self.OnStateChange`
  (params (newState :type "CameraState Enum" :default "kSeeking"))
  (switch `CameraState` newState
    (:`kSeeking`
      (goto _label))
    (:`kAnalyzing`
      (`MaterialInstanceDynamic.SetVectorParameterValue` (`self.DecalMaterial`) "Color" (struct :`R` 1.0 :`G` 0.828312 :`A` 1.0)))
    (:`kAlarm`
      (`MaterialInstanceDynamic.SetVectorParameterValue` (`self.DecalMaterial`) "Color" (struct :`R` 1.0 :`B` 0.025802 :`A` 1.0))
      (`self.ShockPlayer`))))

(event `self.SurveillanceCone.OnComponentBeginOverlap`
  (params (OverlappedComponent :type "PrimitiveComponent Object Reference") (OtherActor :type "Actor Object Reference") (OtherComp :type "PrimitiveComponent Object Reference") (OtherBodyIndex :type Integer) (bFromSweep :type Boolean) (SweepResult :type "HitResult Structure (by ref)"))
  (if (`self.ActorHasTag` OtherActor "Player")
    (set `self.detectedPlayer` OtherActor)))

(event `self.SurveillanceCone.OnComponentEndOverlap`
  (params (OverlappedComponent :type "PrimitiveComponent Object Reference") (OtherActor :type "Actor Object Reference") (OtherComp :type "PrimitiveComponent Object Reference") (OtherBodyIndex :type Integer))
  (if (`self.ActorHasTag` OtherActor "Player")
    (set `self.detectedPlayer` null)))

(event `self.OnRaiseAlarm`
  (`KismetSystemLibrary.PrintString` "Alarm")
  (`self.AlarmDispatch`))

(fn `EndShockPlayer`
  (`SceneComponent.SetVisibility` (`self.ElectricShock`) false false))

(fn `ShockPlayer`
  (bind _detectedplayer (`self.detectedPlayer`))
  (bind _electricshock (`self.ElectricShock`))
  (`|ExecutionSequence`
    (:`then_0`
      ;[1 1 1] Electric shock from camera to player
      (`FXSystemComponent.SetActorParameter` _electricshock "Endpoint" _detectedplayer)
      (`SceneComponent.SetVisibility` _electricshock true false))
    (:`then_1`
      ;[1 1 1] Shock burst in player
      (bind _returnvalue (`|SpawnActorFromClass` "/Game/ElectricShock/ElectricShockBurstBP.ElectricShockBurstBP_C" (`self.GetTransform` _detectedplayer) "Undefined" "OverrideRootScale" null null))
      (`FXSystemComponent.SetActorParameter` (`/Game/ElectricShock/ElectricShockBurstBP.ElectricityBurst` _returnvalue) "Center" _detectedplayer))))

(fn `UserConstructionScript`)